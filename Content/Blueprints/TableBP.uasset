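; Table actor that builds a resizable box tabletop from a procedural mesh, with a rectangular spline path around it.
; UpdateMesh generates the thin box for a given size, stores that size and moves the Corner component to match.
; UpdateSpline adds linear points forming a closed loop slightly outside the table edges.
; The construction script resets to a default square, rebuilds both and enables spline debug drawing; the event graph is empty.
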(event EventBeginPlay)

(event Collision|EventActorBeginOverlap
  (params (OtherActor :type Actor%20Object%20Reference)))

(event EventTick
  (params (DeltaSeconds :type Float%20%28single-precision%29)))

(fn ConstructionScript
  (bind _spline (Variables|Default|GetSpline))
  (bind _output_get (Variables|Default|Setsize "(X=40.000000,Y=40.000000)"))
  (CallFunction|UpdateMesh _output_get)
  (Transformation|SetRelativeLocation (Variables|Default|GetCorner) "40.000000,40.000000, 0" false false)
  (Spline|ClearSplinePoints _spline true)
  (CallFunction|UpdateSpline)
  (Class|SplineComponent|SetDrawDebug _spline true))

(fn UpdateMesh
  (params (tableSize :type Vector%202D%20Structure))
  (bind _proceduralmesh (Variables|Default|GetProceduralMesh))
  (bind (_vertices _triangles _normals _uvs _tangents) (Class|KismetProceduralMeshLibrary|GenerateBoxMesh (Math|Conversions|ToVector(Vector2D) tableSize 3.0)))
  (Class|ProceduralMeshComponent|CreateMeshSectionLinearColor _proceduralmesh 0 _vertices _triangles _normals _uvs 0 0 0 0 _tangents false)
  (Variables|Default|SetDefaultSceneRoot _proceduralmesh)
  (bind _output_get (Variables|Default|Setsize tableSize))
  (Transformation|SetRelativeLocation (Variables|Default|GetCorner) (Math|Conversions|ToVector(Vector2D) _output_get) false false))

(fn UpdateSpline
  (bind _returnvalue (Math|Vector|MakeVector 1.0 1.0 1.0))
  (bind _spline (Variables|Default|GetSpline))
  (bind _size (Variables|Default|Getsize))
  (bind _returnvalue_2 (+ _size "(X=10.000000,Y=10.000000)"))
  (for (_array_element _array_index) (Utilities|Array|MakeArray _returnvalue (Math|Vector|MakeVector -1.0 1.0 1.0) (Math|Vector|MakeVector -1.0 -1.0 1.0) (Math|Vector|MakeVector 1.0 -1.0 1.0) _returnvalue)
    (Spline|AddSplinePoint _spline (* _array_element (Math|Vector|MakeVector (.x _returnvalue_2) (.y _returnvalue_2) 0.0)) "Local" true)
    (Spline|SetSplinePointType _spline _array_index "Linear" true)))