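; MousePlayerControllerBP lets the player resize a TableBP by clicking it and dragging with the mouse.
; Left click traces under the cursor to store the table and hit point, and release ends the drag.
; While held, Tick intersects the cursor ray with the horizontal plane at the hit height.
; That point's offset from the table origin becomes the new size for UpdateMesh, gated by a size-difference check.
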(event EventBeginPlay)

(event EventTick
  (params (DeltaSeconds :type Float%20%28single-precision%29))
  (bind (_worldlocation _worlddirection _returnvalue) (Game|Player|ConvertMouseLocationToWorldSpace))
  (bind _table (Variables|Default|Gettable))
  (bind _defaultsceneroot (Variables|/Game/Blueprints/TableBP.TableBP_C|GetDefaultSceneRoot _table))
  (bind _returnvalue_2 (Transformation|GetWorldLocation _defaultsceneroot))
  (if (Variables|Default|GetcornerPressed)
    (if _returnvalue
      (bind _coordinates (CallFunction|FindCoordinatesinZPlane _worldlocation _worlddirection (.z (Variables|Default|GethitLocation))))
      (Utilities|IsValid _table
        (:Is%20Valid
          (if (|Sizedifference>=2,5 _table (- _coordinates (Math|Vector2D|MakeVector2D (.x _returnvalue_2) (.y _returnvalue_2))))
            (Default|UpdateMesh _table (- _coordinates (Math|Vector2D|MakeVector2D (.x _returnvalue_2) (.y _returnvalue_2))))))))))

(event Input|MouseEvents|LeftMouseButton
  (params (Key :type Key%20Structure :default "None"))
  (bind (_worldlocation _worlddirection) (Game|Player|ConvertMouseLocationToWorldSpace))
  (:Pressed
    (bind (_outhit _returnvalue) (Collision|LineTraceByChannel _worldlocation (+ _worldlocation (* _worlddirection (Math|Float|MakeLiteralFloat 1e+03))) "TraceTypeQuery1" false 0 "None"))
    (bind _astable_bp (Utilities|Casting|CastToTableBP (.HitActor (Collision|BreakHitResult _outhit))))
    (Variables|Default|Settable _astable_bp)
    (Variables|Default|SethitLocation (.ImpactPoint (Collision|BreakHitResult _outhit)))
    (Variables|Default|SetcornerPressed _returnvalue))
  (:Released
    (Variables|Default|SetcornerPressed false)))

(fn ConstructionScript)

(fn FindCoordinatesinZPlane
  (params (location :type Vector) (direction :type Vector) (z%20value :type Float%20%28single-precision%29))
  (bind _returnvalue (- z%20value (.z location)))
  (bind _returnvalue_2 (Math|Float|SafeDivide _returnvalue (.z direction)))
  (return (Math|Vector2D|MakeVector2D (+ (.x location) (* (.x direction) _returnvalue_2)) (+ (.y location) (* (.y direction) _returnvalue_2)))))